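; BP_VA_Character is a character Blueprint with keyboard shortcuts for companion attachment, phase switching and quitting.
; J calls AttachCompanion, and Escape quits the game.
; K cycles CurrentPhase through four phases in a loop, prints the new phase, then calls CheckPhases.
; AttachCompanion and CheckPhases are defined outside these graphs, and Tick and the construction script are empty.
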(event `self.ReceiveTick`
  (params (DeltaSeconds :type "Float (single-precision)")))

(event `Key|J`
  (params (Key :type "Key Structure"))
  (:`Pressed`
    (`self.AttachCompanion`)))

(event `Key|K`
  (params (Key :type "Key Structure"))
  (:`Pressed`
    (switch `EVA_Phase` (`self.CurrentPhase`)
      (:`Phase1`
        (set `self.CurrentPhase` "Phase2"))
      (:`Phase2`
        (set `self.CurrentPhase` "Phase3"))
      (:`Phase3`
        (set `self.CurrentPhase` "Phase4"))
      (:`Phase4`
        (set `self.CurrentPhase` "Phase1")))
    (`KismetSystemLibrary.PrintString` (`KismetStringLibrary.Concat_StrStr` "Change to " "" (`|GetEnumeratorNameAsString` (`self.CurrentPhase`))))
    (`self.CheckPhases`)))

(event `Key|Escape`
  (params (Key :type "Key Structure"))
  (:`Pressed`
    (`KismetSystemLibrary.QuitGame` null "Quit")))

(fn `UserConstructionScript`)