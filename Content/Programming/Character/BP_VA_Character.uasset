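; BP_VA_Character is a character Blueprint that creates the player HUD and connects companion actions to it.
; Show, hide and selection events drive the companion widget's animations, cooldown UI and button highlight on the stored HUD reference.
; Hard-wired keys attach the companion and refresh the HUD, cycle through four phases with an on-screen print before CheckPhases, or quit the game.
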(event `self.ReceiveBeginPlay`
  (bind _returnvalue (`|CreateWidget` "/Game/Programming/Widgets/WBP_PlayerHUD.WBP_PlayerHUD_C" (`GameplayStatics.GetPlayerController` 0)))
  (bind _output_get (set `self.PlayerHUDRef` _returnvalue))
  (`UserWidget.AddToViewport` _output_get 0))

(event `self.ReceiveTick`
  (params (DeltaSeconds :type "Float (single-precision)")))

(event `Key|J`
  (params (Key :type "Key Structure"))
  (:`Pressed`
    (`self.AttachCompanion`)
    (`/Game/Programming/Widgets/WBP_PlayerHUD.UpdateWidget` (`self.PlayerHUDRef`))))

(event `Key|K`
  (params (Key :type "Key Structure"))
  (:`Pressed`
    (switch `EVA_Phase` (`self.CurrentPhase`)
      (:`Phase1`
        (set `self.CurrentPhase` "Phase2"))
      (:`Phase2`
        (set `self.CurrentPhase` "Phase3"))
      (:`Phase3`
        (set `self.CurrentPhase` "Phase4"))
      (:`Phase4`
        (set `self.CurrentPhase` "Phase1")))
    (`KismetSystemLibrary.PrintString` (`KismetStringLibrary.Concat_StrStr` "Change to " "" (`|GetEnumeratorNameAsString` (`self.CurrentPhase`))))
    (`self.CheckPhases`)))

(event `Key|Escape`
  (params (Key :type "Key Structure"))
  (:`Pressed`
    (`KismetSystemLibrary.QuitGame` null "Quit")))

(event `self.ShowCompaWidget`
  ;[0 1 0.9103 0.5] Compa Widget
  (`/Game/Programming/Widgets/WBP_PlayerHUD.PlayCompaAnim_In` (`self.PlayerHUDRef`)))

(event `self.HideCompaWidget`
  (bind _playerhudref (`self.PlayerHUDRef`))
  ;[0 1 0.9103 0.5] Compa Widget
  (`/Game/Programming/Widgets/WBP_PlayerHUD.PlayCompaAnim_Out` _playerhudref)
  (`/Game/Programming/Widgets/WBP_PlayerHUD.SetUICD` _playerhudref))

(event `self.UpdateCompaSelectedButton`
  (params (OrderIndex :type Integer))
  ;[0 1 0.9103 0.5] Compa Widget
  (`/Game/Programming/Widgets/WBP_PlayerHUD.HighlightSelectedButton` (`self.PlayerHUDRef`) OrderIndex))

(fn `UserConstructionScript`)